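; TestPawn is a test selectable pawn that joins team 1 on BeginPlay and can be ordered to move by AI.
; It extends parent selection and action logic, hiding its selection circle at start and toggling it as selection is gained or lost.
; Triggered AI actions send the pawn to the given location with AIMoveTo.
; Debug prints in both selection overrides are disconnected.
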(event EventBeginPlay
  (|CallParentFunction)
  (Class|SURVCharacter|SetTeamNum 1)
  (Rendering|SetVisibility (Variables|Default|GetSelectionSircle) false false))

(event EventTriggerAIAction
  (params (ActionLocation :type Vector%20%28by%20ref%29 :default "0, 0, 0"))
  (|CallParentFunction ActionLocation)
  (AI|AIMoveTo self ActionLocation 0 5.0 false))

(fn ConstructionScript)

(fn OnSelectionLost
  (params (NewPosition :type Vector%20%28by%20ref%29 :default "0, 0, 0") (NewActor :type Actor%20Object%20Reference))
  (bind _returnvalue (|CallParentFunction NewPosition NewActor))
  (Rendering|SetVisibility (Variables|Default|GetSelectionSircle) false false)
  (return _returnvalue))

(fn OnSelectionGained
  (bind _returnvalue (|CallParentFunction))
  (Rendering|SetVisibility (Variables|Default|GetSelectionSircle) true false)
  (return _returnvalue))